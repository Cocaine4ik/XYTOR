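; BP_DialogueCharacter_Dev is a dialogue character that starts a conversation when another actor enters its Box trigger.
; On begin overlap, it copies the DialogueGraph from its ACDialogue component to the overlapping actor's AC_DialogueHandler and calls BeginDialogue.
; On end overlap, it calls EndDialogue on that handler, with no validity check on the component lookup in either event.
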(event `self.ReceiveBeginPlay`
  (`parent.ReceiveBeginPlay`))

(event `self.Box.OnComponentBeginOverlap`
  (params (OverlappedComponent :type "PrimitiveComponent Object Reference") (OtherActor :type "Actor Object Reference") (OtherComp :type "PrimitiveComponent Object Reference") (OtherBodyIndex :type Integer) (bFromSweep :type Boolean) (SweepResult :type "HitResult Structure (by ref)"))
  (bind _returnvalue (`self.GetComponentByClass` OtherActor "/Script/XYTOR.AC_DialogueHandler"))
  (set `AC_Dialogue.DialogueGraph` (`AC_Dialogue.DialogueGraph` (`self.AC_Dialogue`)) _returnvalue)
  (`AC_DialogueHandler.BeginDialogue` _returnvalue))

(event `self.Box.OnComponentEndOverlap`
  (params (OverlappedComponent :type "PrimitiveComponent Object Reference") (OtherActor :type "Actor Object Reference") (OtherComp :type "PrimitiveComponent Object Reference") (OtherBodyIndex :type Integer))
  (`AC_DialogueHandler.EndDialogue` (`self.GetComponentByClass` OtherActor "/Script/XYTOR.AC_DialogueHandler")))

(fn `UserConstructionScript`
  (`parent.UserConstructionScript`))