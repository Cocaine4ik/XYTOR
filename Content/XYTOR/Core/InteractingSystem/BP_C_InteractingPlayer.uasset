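; Player pawn Blueprint that feeds nearby actors to the interaction system.
; On BeginPlay it casts its controller to PC_Interaction and stores it, printing an on-screen error if the controller is the wrong type.
; Begin and end overlap events on its ItemsOverlaping component call AddActor and RemoveActor on that controller, which receives every overlapping actor without filtering here.
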(event `self.ReceiveBeginPlay`
  (bind _aspc_interaction (cast `PC_Interaction` (`self.GetController`))
    (:`then`
      (set `self.InteractingController` _aspc_interaction))
    (:`CastFailed`
      (`KismetSystemLibrary.PrintString` "Incorrect controller for interacting" true true (struct :`R` 1.0 :`B` 0.045438 :`A` 1.0) 60.0))))

(event `self.ItemsOverlaping.OnComponentBeginOverlap`
  (params (OverlappedComponent :type "PrimitiveComponent Object Reference") (OtherActor :type "Actor Object Reference") (OtherComp :type "PrimitiveComponent Object Reference") (OtherBodyIndex :type Integer) (bFromSweep :type Boolean) (SweepResult :type "HitResult Structure (by ref)"))
  (`PC_Interaction.AddActor` (`self.InteractingController`) OtherActor))

(event `self.ItemsOverlaping.OnComponentEndOverlap`
  (params (OverlappedComponent :type "PrimitiveComponent Object Reference") (OtherActor :type "Actor Object Reference") (OtherComp :type "PrimitiveComponent Object Reference") (OtherBodyIndex :type Integer))
  (`PC_Interaction.RemoveActor` (`self.InteractingController`) OtherActor))

(fn `UserConstructionScript`
  (`parent.UserConstructionScript`))