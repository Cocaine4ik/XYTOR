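; Player controller Blueprint for the detective character that toggles evidence detection with the right mouse button.
; Pressing the button casts the player pawn to BP_CH_Detective and turns evidence detecting on, and releasing it turns it off.
; The BeginPlay and Tick events are disabled, and the construction script only calls the parent.
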(event `Key|RightMouseButton`
  (params (Key :type "Key Structure"))
  (:`Pressed`
    (bind _asbp_ch_detective (cast `/Game/XYTOR/Core/Detective/BP_CH_Detective` (`GameplayStatics.GetPlayerPawn` 0)))
    (`/Game/XYTOR/Core/Detective/BP_CH_Detective.SetEvidencesDetecting` _asbp_ch_detective true))
  (:`Released`
    (bind _asbp_ch_detective_2 (cast `/Game/XYTOR/Core/Detective/BP_CH_Detective` (`GameplayStatics.GetPlayerPawn` 0)))
    (`/Game/XYTOR/Core/Detective/BP_CH_Detective.SetEvidencesDetecting` _asbp_ch_detective_2 false)))

(fn `UserConstructionScript`
  (`parent.UserConstructionScript`))