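; BP_DialogueCharacter_Dev is a dialogue character Blueprint that exposes its ACDialogue component to an interaction system.
; GetHandlers adds ACDialogue to the Handlers list and returns it, and GetInteractingText returns the interacting text stored on that component.
; BeginPlay and the construction script only call their parent versions, so the Blueprint adds no other logic of its own.
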(event `self.ReceiveBeginPlay`
  (`parent.ReceiveBeginPlay`))

(fn `GetHandlers`
  (returns (ReturnValue :type "Array of AC_Interact Object Reference"))
  (locals (Handlers :type "Array of AC_Interact Object Reference"))
  (bind _handlers (`local.Handlers`))
  (`KismetArrayLibrary.Array_Add` _handlers (`self.AC_Dialogue`))
  (return _handlers))

(fn `GetInteractingText`
  (returns (ReturnValue :type Text))
  (return (`AC_Interact.InteractingText` (`self.AC_Dialogue`))))

(fn `UserConstructionScript`
  (`parent.UserConstructionScript`))